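; Mod actor that adds a bulk fertilize button to the farm field details window.
; Mouse releases and window button clicks show a waiter widget linked to this actor; OnClickCheck finds the window, injects the button and refreshes its crop label.
; Clicking it points a hidden helper widget's Context at each field within the configured range, fertilizing same-crop fields, or setting all seeded fields to fallow, derocked and fertilized when fallow is selected.
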(event Custom|OnClickCheck
  (bind _returnvalue (Utilities|String|Append "resource." ""))
  (bind _helper (Variables|Default|GetHelper))
  (bind _state (Variables|/Game/Mods/Fertilizer/WBP_FieldHelper.WBP_FieldHelper_C|GetState _helper))
  (bind _activeseeds (Utilities|Struct|BreakFarmFieldUIState _state))
  (bind _returnvalue_2 (Utilities|String|ToString(Name) _activeseeds))
  (bind _returnvalue_3 (Utilities|Enum|Equal(Enum) _returnvalue_2 "wood"))
  (bind _returnvalue_4 (Utilities|String|SelectString "trees" _returnvalue_2 _returnvalue_3))
  (bind _returnvalue_5 (Utilities|String|Append _returnvalue _returnvalue_4))
  (bind _returnvalue_6 (Utilities|String|StringToName _returnvalue_5))
  (bind _returnvalue_7 (Class|LocManager|GetWordfromKey _returnvalue_6))
  (Variables|Default|SetWin 0)
  (bind _foundwidgets (Widget|GetAllWidgetsOfClass self "/Script/ProjectArco.UI_FarmFieldDetails"))
  (for _array_element _foundwidgets
    (if (and (!= _array_element (Variables|Default|GetHelper)) (Widget|IsVisible _array_element))
      (Variables|Default|SetWin _array_element)))
  (if (and (Utilities|IsValid (Variables|Default|GetWin)) (!= (Variables|Default|GetWin) (Variables|Default|GetInjected)))
    (if (Variables|Default|GetDebug)
      (Class|ModAPI|LogMessage (Class|ModAPI|GetModAPI) (Utilities|String|Append (Utilities|String|Append (Utilities|String|Append (Utilities|String|Append (Utilities|String|Append "Fertilizer: new crop field window " "") (Utilities|GetDisplayName (Variables|Default|GetWin))) " [") (Utilities|GetClassDisplayName (Utilities|GetClass (Variables|Default|GetWin)))) "]") true))
    (Variables|Default|SetTarget 0)
    (bind _returnvalue_8 (Class|NaviUi|FindDecendentsOfClasses (Variables|Default|GetWin) (Utilities|Array|MakeArray "/Script/UMG.VerticalBox") false))
    (for _array_element_2 _returnvalue_8
      (if (or (Utilities|Enum|Equal(Enum) (Utilities|GetDisplayName (Widget|GetParent _array_element_2)) "contents") (not (Utilities|IsValid (Variables|Default|GetTarget))))
        (bind _aspanel_widget (Utilities|Casting|CastToPanelWidget _array_element_2))
        (Variables|Default|SetTarget _aspanel_widget)))
    (if (Utilities|IsValid (Variables|Default|GetTarget))
      (bind _returnvalue_9 (Widget|Panel|AddChild (Variables|Default|GetTarget) (Variables|Default|GetFertButton)))
      (Variables|Default|SetInjected (Variables|Default|GetWin))
      (if (Variables|Default|GetDebug)
        (Class|ModAPI|LogMessage (Class|ModAPI|GetModAPI) (Utilities|String|Append (Utilities|String|Append (Utilities|String|Append (Utilities|String|Append "Fertilizer: button added to " "") (Utilities|GetDisplayName (Variables|Default|GetTarget))) " slot ") (Utilities|GetClassDisplayName (Utilities|GetClass _returnvalue_9))) true))
      (bind _asvertical_box_slot (Utilities|Casting|CastToVerticalBoxSlot _returnvalue_9)
        (:then
          (Layout|GridSlot|SetHorizontalAlignment _asvertical_box_slot "HAlign_Center")
          (Layout|BorderSlot|SetPadding _asvertical_box_slot "(Left=0.000000,Top=12.000000,Right=0.000000,Bottom=4.000000)" :!class /Script/UMG.VerticalBoxSlot)
          (bind _returnvalue_10 (Class|NaviUi|FindDecendentsOfClasses (Variables|Default|GetWin) (Utilities|Array|MakeArray "/Script/UMG.Button") false))
          (for _array_element_3 _returnvalue_10
            (bind _asbutton (Utilities|Casting|CastToButton _array_element_3))
            (if (!= _asbutton (Variables|/Game/Mods/Fertilizer/WBP_FertButton.WBP_FertButton_C|GetBtn (Variables|Default|GetFertButton)))
              (EventDispatchers|BindEventtoOnClicked _asbutton (delegate Custom|OnWindowButton)))))
        (:CastFailed
          _))
      (bind _asarco_widget_base (Utilities|Casting|CastToArcoWidgetBase (Variables|Default|GetWin) :!label _label))
      (Class|KismetSystemLibrary|SetObjectPropertybyName _helper "Context" (Variables|/Script/ProjectArco.ArcoWidgetBase|GetContext _asarco_widget_base))
      (Default|ReadState _helper)
      (bind _returnvalue_11 (Class|ModAPI|ReadModOptionValue (Class|ModAPI|GetModAPI) "Fertilizer_Range" "30"))
      (if (Utilities|Name|NotEqual(Name) _activeseeds "None")
        (Rendering|Components|TextRender|SetText (Variables|/Game/Mods/Fertilizer/WBP_FertButton.WBP_FertButton_C|GetLabel (Variables|Default|GetFertButton)) (Utilities|Text|ToText(String) (Utilities|String|SelectString (Utilities|String|Append (Utilities|String|Append (Utilities|String|Append "Fallow + derock + fertilize all within " "") _returnvalue_11) " tiles") (Utilities|String|Append (Utilities|String|Append (Utilities|String|Append (Utilities|String|Append (Utilities|String|Append "Fertilize all " "") (Utilities|String|SelectString _returnvalue_2 _returnvalue_7 (Utilities|Array|IsEmpty _returnvalue_7))) " within ") _returnvalue_11) " tiles") (Utilities|Name|Equal(Name) _activeseeds "fallow"))))
        (Widget|SetIsEnabled (Variables|Default|GetFertButton) true)
        (else
          (Rendering|Components|TextRender|SetText (Variables|/Game/Mods/Fertilizer/WBP_FertButton.WBP_FertButton_C|GetLabel (Variables|Default|GetFertButton)) (Utilities|Text|ToText(String) (Utilities|String|Append "No crop chosen" "")))
          (Widget|SetIsEnabled (Variables|Default|GetFertButton) false)))
      (elif (Variables|Default|GetDebug)
        (Class|ModAPI|LogMessage (Class|ModAPI|GetModAPI) "Fertilizer: no VerticalBox in the window, cannot add the button" true)))
    (elif (Utilities|IsValid (Variables|Default|GetWin))
      (goto _label))))

(event Custom|OnFertClick
  (bind _helper (Variables|Default|GetHelper))
  (bind _helper_2 (Variables|Default|GetHelper))
  (bind _state (Variables|/Game/Mods/Fertilizer/WBP_FieldHelper.WBP_FieldHelper_C|GetState _helper_2))
  (bind _state_2 (Variables|/Game/Mods/Fertilizer/WBP_FieldHelper.WBP_FieldHelper_C|GetState _helper))
  (bind _activeseeds (Utilities|Struct|BreakFarmFieldUIState _state))
  (bind (_activeseeds_2 _bfertilizeractive _bremovingrocksactive) (Utilities|Struct|BreakFarmFieldUIState _state_2))
  (bind _returnvalue (not _bfertilizeractive))
  (bind _returnvalue_2 (not _bremovingrocksactive))
  (bind _returnvalue_3 (Utilities|Name|NotEqual(Name) _activeseeds_2 "fallow"))
  (bind _asarco_widget_base (Utilities|Casting|CastToArcoWidgetBase (Variables|Default|GetInjected)))
  (Variables|Default|SetSel (Variables|/Script/ProjectArco.ArcoWidgetBase|GetContext _asarco_widget_base))
  (Variables|Default|SetChanged 0)
  (bind _returnvalue_4 (Class|ModAPI|ReadModOptionValue (Class|ModAPI|GetModAPI) "Fertilizer_Range" "30"))
  (Variables|Default|SetRange (Math|Conversions|ToInteger(Byte) _returnvalue_4))
  (bind _asgrid_actor (Utilities|Casting|CastToGridActor (Variables|Default|GetSel))
    (:then
      (Variables|Default|SetSelRoot (Math|Conversions|ToVector(Float) (Utilities|Struct|BreakGridFootprint (Variables|/Script/ProjectArco.GridActor|GetliveFootprint _asgrid_actor))))
      (Class|KismetSystemLibrary|SetObjectPropertybyName _helper_2 "Context" (Variables|Default|GetSel))
      (Default|ReadState _helper_2)
      (Variables|Default|SetSelSeeds _activeseeds)
      (if (Utilities|Name|NotEqual(Name) _activeseeds "None")
        (if (Variables|Default|GetDebug)
          (Class|ModAPI|LogMessage (Class|ModAPI|GetModAPI) (Utilities|String|Append (Utilities|String|Append (Utilities|String|Append (Utilities|String|Append "Fertilizer: button pressed, crop=" "") (Utilities|String|ToString(Name) _activeseeds)) " range=") (Utilities|String|ToString(Integer) (Math|Conversions|ToInteger(Byte) _returnvalue_4))) true))
        (bind _asactor (Utilities|Casting|CastToActorClass (Utilities|GetClass (Variables|Default|GetSel))))
        (bind _outactors (Actor|GetAllActorsOfClass self _asactor))
        (for _array_element _outactors
          (bind _asgrid_actor_2 (Utilities|Casting|CastToGridActor _array_element))
          (if (<= (Math|Vector|VectorLengthXY (- (Math|Conversions|ToVector(Float) (Utilities|Struct|BreakGridFootprint (Variables|/Script/ProjectArco.GridActor|GetliveFootprint _asgrid_actor_2))) (Variables|Default|GetSelRoot))) (Math|Conversions|ToFloat(Integer) (Variables|Default|GetRange)))
            (Class|KismetSystemLibrary|SetObjectPropertybyName _helper "Context" _array_element)
            (Default|ReadState _helper)
            (if (or (and (not (Utilities|Name|Equal(Name) (Variables|Default|GetSelSeeds) "fallow")) (and (Utilities|Name|Equal(Name) _activeseeds_2 (Variables|Default|GetSelSeeds)) _returnvalue)) (and (Utilities|Name|Equal(Name) (Variables|Default|GetSelSeeds) "fallow") (and (or (or _returnvalue _returnvalue_2) _returnvalue_3) (Utilities|Name|NotEqual(Name) _activeseeds_2 "None"))))
              (if _returnvalue
                (Default|ApplyFertilizer _helper))
              (if (and (Utilities|Name|Equal(Name) (Variables|Default|GetSelSeeds) "fallow") _returnvalue_2)
                (Default|ApplyRocks _helper))
              (if (and (Utilities|Name|Equal(Name) (Variables|Default|GetSelSeeds) "fallow") _returnvalue_3)
                (Default|ApplyFallow _helper))
              (Variables|Default|SetChanged (+ (Variables|Default|GetChanged) 1))
              (if (Variables|Default|GetDebug)
                (Class|ModAPI|LogMessage (Class|ModAPI|GetModAPI) (Utilities|String|Append (Utilities|String|Append (Utilities|String|Append (Utilities|String|Append "Fertilizer:   changed field at " "") (Utilities|String|ToString(Integer) (Utilities|Struct|BreakGridFootprint (Variables|/Script/ProjectArco.GridActor|GetliveFootprint _asgrid_actor_2)))) " distance ") (Utilities|String|ToString(Float) (Math|Vector|VectorLengthXY (- (Math|Conversions|ToVector(Float) (Utilities|Struct|BreakGridFootprint (Variables|/Script/ProjectArco.GridActor|GetliveFootprint _asgrid_actor_2))) (Variables|Default|GetSelRoot))))) true)))))
        (if (Variables|Default|GetDebug)
          (Class|ModAPI|LogMessage (Class|ModAPI|GetModAPI) (Utilities|String|Append (Utilities|String|Append "Fertilizer: done, fields switched on: " "") (Utilities|String|ToString(Integer) (Variables|Default|GetChanged))) true))
        (Rendering|Components|TextRender|SetText (Variables|/Game/Mods/Fertilizer/WBP_FertButton.WBP_FertButton_C|GetLabel (Variables|Default|GetFertButton)) (Utilities|Text|ToText(String) (Utilities|String|SelectString (Utilities|String|Append (Utilities|String|Append (Utilities|String|Append "Done: " "") (Utilities|String|ToString(Integer) (Variables|Default|GetChanged))) " fields set to fallow, derocked and fertilized") (Utilities|String|Append (Utilities|String|Append (Utilities|String|Append (Utilities|String|Append (Utilities|String|Append "Done: " "") (Utilities|String|ToString(Integer) (Variables|Default|GetChanged))) " more ") (Utilities|String|SelectString (Utilities|String|ToString(Name) (Variables|Default|GetSelSeeds)) (Class|LocManager|GetWordfromKey (Utilities|String|StringToName (Utilities|String|Append (Utilities|String|Append "resource." "") (Utilities|String|SelectString "trees" (Utilities|String|ToString(Name) (Variables|Default|GetSelSeeds)) (Utilities|Enum|Equal(Enum) (Utilities|String|ToString(Name) (Variables|Default|GetSelSeeds)) "wood"))))) (Utilities|Array|IsEmpty (Class|LocManager|GetWordfromKey (Utilities|String|StringToName (Utilities|String|Append (Utilities|String|Append "resource." "") (Utilities|String|SelectString "trees" (Utilities|String|ToString(Name) (Variables|Default|GetSelSeeds)) (Utilities|Enum|Equal(Enum) (Utilities|String|ToString(Name) (Variables|Default|GetSelSeeds)) "wood")))))))) " fields fertilized") (Utilities|Name|Equal(Name) (Variables|Default|GetSelSeeds) "fallow"))))
        (elif (Variables|Default|GetDebug)
          (Class|ModAPI|LogMessage (Class|ModAPI|GetModAPI) "Fertilizer: selected field has no seed choice, nothing to do" true))))
    (:CastFailed
      (if (Variables|Default|GetDebug)
        (Class|ModAPI|LogMessage (Class|ModAPI|GetModAPI) "Fertilizer: the window has no field tile selected" true)))))

(event Custom|OnLoaded
  (bind _returnvalue (Game|GetPlayerController 0))
  (if (not (Variables|Default|GetReady))
    (if (Utilities|IsValid (Game|GetPlayerController 0))
      (Variables|Default|SetReady true)
      (bind _returnvalue_2 (Class|ModAPI|ReadModTextFile (Class|ModAPI|GetModAPI) "FertilizerConfig" "debug"))
      (Variables|Default|SetDebug (not (Utilities|Array|IsEmpty _returnvalue_2)))
      (if (Variables|Default|GetDebug)
        (Class|ModAPI|LogMessage (Class|ModAPI|GetModAPI) "Fertilizer ready" true))
      (Input|EnableInput self _returnvalue)
      (bind _returnvalue_3 (UserInterface|CreateWidget "/Game/Mods/Fertilizer/WBP_FieldHelper.WBP_FieldHelper_C" _returnvalue))
      (Variables|Default|SetHelper _returnvalue_3)
      (bind _returnvalue_4 (UserInterface|CreateWidget "/Game/Mods/Fertilizer/WBP_FertButton.WBP_FertButton_C" _returnvalue))
      (Variables|Default|SetFertButton _returnvalue_4)
      (EventDispatchers|BindEventtoOnClicked (Variables|/Game/Mods/Fertilizer/WBP_FertButton.WBP_FertButton_C|GetBtn _returnvalue_4) (delegate Custom|OnFertClick))
      (bind _returnvalue_5 (UserInterface|CreateWidget "/Game/Mods/Fertilizer/WBP_ClickWaiter.WBP_ClickWaiter_C" _returnvalue))
      (Variables|Default|SetWaiter _returnvalue_5)
      (Class|KismetSystemLibrary|SetObjectPropertybyName _returnvalue_5 "Owner" self)
      (elif (< (Variables|Default|GetTries) 10)
        (Variables|Default|SetTries (+ (Variables|Default|GetTries) 1))
        (Utilities|Time|SetTimerbyFunctionName self "OnLoaded" 1.0)))))

(event Custom|OnWindowButton
  (bind _waiter (Variables|Default|GetWaiter))
  (if (not (UserInterface|Viewport|IsinViewport _waiter))
    (UserInterface|Viewport|AddtoViewport _waiter 0)))

(event EventBeginPlay
  (bind _returnvalue (Game|GetPlayerController 0))
  (EventDispatchers|BindEventtoOnLoadingFinished (Class|ModAPI|GetModAPI) (delegate Custom|OnLoaded))
  (if (not (Variables|Default|GetReady))
    (if (Utilities|IsValid (Game|GetPlayerController 0))
      (Variables|Default|SetReady true)
      (bind _returnvalue_2 (Class|ModAPI|ReadModTextFile (Class|ModAPI|GetModAPI) "FertilizerConfig" "debug"))
      (Variables|Default|SetDebug (not (Utilities|Array|IsEmpty _returnvalue_2)))
      (if (Variables|Default|GetDebug)
        (Class|ModAPI|LogMessage (Class|ModAPI|GetModAPI) "Fertilizer ready" true))
      (Input|EnableInput self _returnvalue)
      (bind _returnvalue_3 (UserInterface|CreateWidget "/Game/Mods/Fertilizer/WBP_FieldHelper.WBP_FieldHelper_C" _returnvalue))
      (Variables|Default|SetHelper _returnvalue_3)
      (bind _returnvalue_4 (UserInterface|CreateWidget "/Game/Mods/Fertilizer/WBP_FertButton.WBP_FertButton_C" _returnvalue))
      (Variables|Default|SetFertButton _returnvalue_4)
      (EventDispatchers|BindEventtoOnClicked (Variables|/Game/Mods/Fertilizer/WBP_FertButton.WBP_FertButton_C|GetBtn _returnvalue_4) (delegate Custom|OnFertClick))
      (bind _returnvalue_5 (UserInterface|CreateWidget "/Game/Mods/Fertilizer/WBP_ClickWaiter.WBP_ClickWaiter_C" _returnvalue))
      (Variables|Default|SetWaiter _returnvalue_5)
      (Class|KismetSystemLibrary|SetObjectPropertybyName _returnvalue_5 "Owner" self)
      (elif (< (Variables|Default|GetTries) 10)
        (Variables|Default|SetTries (+ (Variables|Default|GetTries) 1))
        (Utilities|Time|SetTimerbyFunctionName self "OnLoaded" 1.0)))))

(event Input|MouseEvents|LeftMouseButton
  (params (Key :type Key%20Structure :default "None"))
  (bind _waiter (Variables|Default|GetWaiter))
  (:Released
    (if (not (UserInterface|Viewport|IsinViewport _waiter))
      (UserInterface|Viewport|AddtoViewport _waiter 0))))

(fn ConstructionScript)